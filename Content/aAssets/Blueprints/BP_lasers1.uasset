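; BP_lasers1 is a laser hazard actor that respawns the first-person character on contact.
; Each tick it traces along its up vector and scales the Root's Z to reach the first blocking hit, or a default length when nothing is hit.
; A Trigger component's begin overlap casts the other actor to BP_FirstPersonCharacter and calls Respawn on it.
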(event `self.ReceiveTick`
  (params (DeltaSeconds :type "Float (single-precision)"))
  (bind _returnvalue (`self.K2_GetActorLocation`))
  (bind (_outhit _returnvalue_2) (`KismetSystemLibrary.LineTraceSingle` _returnvalue (+ _returnvalue (* (`self.GetActorUpVector`) 10000.0)) "TraceTypeQuery1"))
  (`SceneComponent.SetRelativeScale3D` (`self.Root`) (`KismetMathLibrary.MakeVector` 1.0 1.0 (/ (`KismetMathLibrary.SelectFloat` (`.Distance` (`GameplayStatics.BreakHitResult` _outhit)) 8000.0 _returnvalue_2) 186.0))))

(event `self.Trigger.OnComponentBeginOverlap`
  (params (OverlappedComponent :type "PrimitiveComponent Object Reference") (OtherActor :type "Actor Object Reference") (OtherComp :type "PrimitiveComponent Object Reference") (OtherBodyIndex :type Integer) (bFromSweep :type Boolean) (SweepResult :type "HitResult Structure (by ref)"))
  (bind _asbp_first_person_character (cast `/Game/FirstPerson/Blueprints/BP_FirstPersonCharacter` OtherActor))
  (`/Game/FirstPerson/Blueprints/BP_FirstPersonCharacter.Respawn` _asbp_first_person_character))

(fn `UserConstructionScript`)